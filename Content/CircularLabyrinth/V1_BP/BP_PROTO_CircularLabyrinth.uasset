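; Prototype actor that builds a circular labyrinth grid of walls and cells in the construction script, with no path carving yet.
; Concentric rings of chord-scaled HISM segments get radial HISM walls between their corner points.
; Cells, starting from a center cell 0, store walls, points and wrap-around neighbor indices, with debug markers and index labels.
; Two test events hide a chosen ring or radial wall by zero-scaling its instance.
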(event `TestAWall`
  (`InstancedStaticMeshComponent.UpdateInstanceTransform` (`self.HISM_Circle`) (`.Instanceindex_10_3155ACAB45FCBAC9F3F375BB2E59E261` (break `/Game/CircularLabyrinth/V1_BP/S_PROTO_Wall` (`|GetArrayItem` (`self.CircleWalls`) (`self.IndexCircleWallToTest`)))) (`KismetMathLibrary.MakeTransform` (0.0 0.0 0.0) (struct) (0.0 0.0 0.0)) false false false))

(event `TestSubWall`
  (`InstancedStaticMeshComponent.UpdateInstanceTransform` (`self.HISM_Wall`) (`.Instanceindex_10_3155ACAB45FCBAC9F3F375BB2E59E261` (break `/Game/CircularLabyrinth/V1_BP/S_PROTO_Wall` (`|GetArrayItem` (`self.SubWalls`) (`self.IndexSubWallToTest`)))) (`KismetMathLibrary.MakeTransform` (0.0 0.0 0.0) (struct) (0.0 0.0 0.0)) false false false))

(fn `ClearVariables`
  (`KismetArrayLibrary.Array_Clear` (`self.WallNeighbors`))
  (`KismetArrayLibrary.Array_Clear` (`self.TempsWalls`))
  (`KismetArrayLibrary.Array_Clear` (`self.GridPoints`))
  (`KismetArrayLibrary.Array_Clear` (`self.CircleWalls`))
  (`KismetArrayLibrary.Array_Clear` (`self.Cells`))
  (`KismetArrayLibrary.Array_Clear` (`self.SubWalls`)))

(fn `CreateWallsBetweenCircle&WallLoc`
  (for _index (range 1 (`self.CircleCount`))
    (for _index_2 (range (`self.Subdivision`))
      (bind (_instanceindex _wallloc _pointa _pointb) (break `/Game/CircularLabyrinth/V1_BP/S_PROTO_Wall` (`|GetArrayItem` (`self.CircleWalls`) (+ _index_2 (* (- _index 1) (`self.Subdivision`))))))
      (bind (_instanceindex_2 _wallloc_2 _pointa_2 _pointb_2) (break `/Game/CircularLabyrinth/V1_BP/S_PROTO_Wall` (`|GetArrayItem` (`self.CircleWalls`) (+ _index_2 (* _index (`self.Subdivision`))))))
      (bind _returnvalue (/ (+ _pointb _pointb_2) 2.0))
      (bind _returnvalue_2 (`InstancedStaticMeshComponent.AddInstance` (`self.HISM_Wall`) (`KismetMathLibrary.MakeTransform` _returnvalue (`KismetMathLibrary.FindLookAtRotation` _pointb _pointb_2) (`KismetMathLibrary.MakeVector` (/ (`KismetMathLibrary.Vector_Distance` _pointb _pointb_2) 100.0) 1.0 4.0)) true))
      (`KismetArrayLibrary.Array_Add` (`self.SubWalls`) (make `/Game/CircularLabyrinth/V1_BP/S_PROTO_Wall` _returnvalue_2 _returnvalue _pointb _pointb_2)))))

(fn `DEBUG_CellTextIndex`
  (for _array_element (`self.Cells`)
    (bind (_index _neighborscount _cellloc) (break `/Game/CircularLabyrinth/V1_BP/S_PROTO_Cell` _array_element))
    (`InstancedStaticMeshComponent.AddInstance` (`self.DEBUG_HISM`) (`KismetMathLibrary.MakeTransform` _cellloc) true)
    (bind _returnvalue (`AddComponent|NODE_AddTextRenderComponent-0` :`bManualAttachment` true :`RelativeTransform` (`KismetMathLibrary.MakeTransform` (`KismetMathLibrary.MakeVector` (.x _cellloc) (.y _cellloc) (+ (.z _cellloc) 250.0)) (struct :`Pitch` 90.0 :`Yaw` 180.0))))
    (`TextRenderComponent.K2_SetText` _returnvalue (`KismetTextLibrary.Conv_StringToText` (`KismetStringLibrary.Conv_IntToString` _index)))
    (`TextRenderComponent.SetWorldSize` _returnvalue 400.0)
    (`TextRenderComponent.SetHorizontalAlignment` _returnvalue "EHTA_Center")
    (`TextRenderComponent.SetVerticalAlignment` _returnvalue "EVRTA_TextCenter")))

(fn `DrawCircles&Points`
  (for _index (range 1 (+ (`self.CircleCount`) 1))
    (bind _returnvalue (* (`self.Radius`) _index))
    (`self.DrawCircleWithRadius` _returnvalue)
    (`self.DrawPointsWithRadius` _returnvalue)))

(fn `DrawCircleWithRadius`
  (params (`L Radius` :type "Float (double-precision)"))
  (locals (`L Index` :type Integer) (`L Angle Radian` :type "Float (double-precision)" :default 0.0) (`L AngleStepTetaDegrees` :type "Float (double-precision)"))
  (bind _returnvalue (+ (`KismetMathLibrary.MakeVector` (* (`local.L Radius`) (`KismetMathLibrary.Cos` (`local.L Angle Radian`))) (* (`local.L Radius`) (`KismetMathLibrary.Sin` (`local.L Angle Radian`)))) (`self.K2_GetActorLocation`)))
  (set `local.L AngleStepTetaDegrees` (/ 360.0 (`KismetMathLibrary.Conv_IntToDouble` (`self.Subdivision`))))
  (for _index (range (`self.Subdivision`))
    (set `local.L Index` _index)
    (set `local.L Angle Radian` (`KismetMathLibrary.DegreesToRadians` (* (`local.L AngleStepTetaDegrees`) _index)))
    (bind _returnvalue_2 (`InstancedStaticMeshComponent.AddInstance` (`self.HISM_Circle`) (`KismetMathLibrary.MakeTransform` _returnvalue (`KismetMathLibrary.MakeRotator` 0.0 0.0 (* (`local.L AngleStepTetaDegrees`) (`local.L Index`))) (`KismetMathLibrary.MakeVector` 1.0 (/ (* (* 2.0 (`local.L Radius`)) (`KismetMathLibrary.DegSin` (/ (`local.L AngleStepTetaDegrees`) 2.0))) (* (.y (`.Max` (break `Box` (`StaticMesh.GetBoundingBox` (`self.Static Mesh`))))) 2.0)) 4.0)) true))
    (`KismetArrayLibrary.Array_Add` (`self.TempsWalls`) (make `/Game/CircularLabyrinth/V1_BP/S_PROTO_Wall` _returnvalue_2 _returnvalue))))

(fn `DrawPointsWithRadius`
  (params (`L Radius` :type "Float (double-precision)"))
  (locals (`L Index` :type Integer) (`L Angle Radian` :type "Float (double-precision)" :default 0.0) (`L AngleStepThetaDegrees` :type "Float (double-precision)"))
  (bind _returnvalue (+ (`KismetMathLibrary.MakeVector` (* (`local.L Radius`) (`KismetMathLibrary.Cos` (`local.L Angle Radian`))) (* (`local.L Radius`) (`KismetMathLibrary.Sin` (`local.L Angle Radian`)))) (`self.K2_GetActorLocation`)))
  (set `local.L AngleStepThetaDegrees` (/ 360.0 (`KismetMathLibrary.Conv_IntToDouble` (`self.Subdivision`))))
  (for _index (range (`self.Subdivision`))
    (set `local.L Index` _index)
    (set `local.L Angle Radian` (`KismetMathLibrary.DegreesToRadians` (* (`local.L AngleStepThetaDegrees`) (+ _index 0.5))))
    (`InstancedStaticMeshComponent.AddInstance` (`self.DEBUG_HISM`) (`KismetMathLibrary.MakeTransform` _returnvalue (`KismetMathLibrary.MakeRotator` 0.0 0.0 (* (`local.L AngleStepThetaDegrees`) (`local.L Index`))) (1.0 1.0 10.0)) true)
    (`KismetArrayLibrary.Array_Add` (`self.GridPoints`) _returnvalue)))

(fn `FinalCellsSetup`
  (`KismetArrayLibrary.Array_Clear` (`self.Cells`))
  (`self.SetupCell_Index0`)
  (for _array_element (`self.TempsCells`)
    (`KismetArrayLibrary.Array_Add` (`self.Cells`) _array_element)))

(fn `SetIndexCellsNeighbors`
  (locals (Threshold :type Integer))
  (bind _cells (`self.Cells`))
  (bind _newindexneighbors (`self.NewIndexNeighbors`))
  (set `local.Threshold` (`self.Subdivision`))
  (for _index (range 1 (`KismetArrayLibrary.Array_Length` _cells))
    (if (> _index (`local.Threshold`))
      (set `local.Threshold` (+ (`local.Threshold`) (`self.Subdivision`))))
    (bind (_index_2 _neighborscount _cellloc _current _visited _walls _points) (break `/Game/CircularLabyrinth/V1_BP/S_PROTO_Cell` (`|GetArrayItem` _cells _index)))
    (bind _returnvalue (+ _index_2 1))
    (`KismetArrayLibrary.Array_Add` _newindexneighbors (`KismetMathLibrary.SelectInt` (- _index_2 (- (`self.Subdivision`) 1)) _returnvalue (> _returnvalue (`local.Threshold`))))
    (bind _returnvalue_2 (- _index_2 1))
    (`KismetArrayLibrary.Array_Add` _newindexneighbors (`KismetMathLibrary.SelectInt` (`local.Threshold`) _returnvalue_2 (== _returnvalue_2 (- (`local.Threshold`) (`self.Subdivision`)))))
    (bind _returnvalue_3 (- _index_2 (`self.Subdivision`)))
    (`KismetArrayLibrary.Array_Add` _newindexneighbors (`KismetMathLibrary.SelectInt` 0 _returnvalue_3 (< _returnvalue_3 0)))
    (bind _returnvalue_4 (+ _index_2 (`self.Subdivision`)))
    (if (not (> _returnvalue_4 (- (`KismetArrayLibrary.Array_Length` (`self.Cells`)) 1)))
      (`KismetArrayLibrary.Array_Add` _newindexneighbors _returnvalue_4))
    (`KismetArrayLibrary.Array_Add` (`self.TempsCells`) (make `/Game/CircularLabyrinth/V1_BP/S_PROTO_Cell` _index_2 _neighborscount _cellloc _current _visited _walls _points _newindexneighbors))
    (`KismetArrayLibrary.Array_Clear` (`self.NewIndexNeighbors`))))

(fn `SetupCell_Index0`
  (`KismetArrayLibrary.Array_Add` (`self.Cells`) (make `/Game/CircularLabyrinth/V1_BP/S_PROTO_Cell` 0 (`self.Subdivision`) (`self.K2_GetActorLocation`))))

(fn `SetWalls&PointsToCells`
  (bind _wallneighbors (`self.WallNeighbors`))
  (bind _wallneighbors_2 (`self.WallNeighbors`))
  (bind _tempspoints (`self.TempsPoints`))
  (for _index (range 1 (`self.CircleCount`))
    (for _index_2 (range (`self.Subdivision`))
      (bind _returnvalue (* (- _index 1) (`self.Subdivision`)))
      (bind _returnvalue_2 (+ _index_2 _returnvalue))
      (bind _output (`|GetArrayItem` (`self.CircleWalls`) _returnvalue_2))
      (`KismetArrayLibrary.Array_Add` _wallneighbors_2 _output)
      (bind _output_2 (`|GetArrayItem` (`self.CircleWalls`) (+ _index_2 (* _index (`self.Subdivision`)))))
      (`KismetArrayLibrary.Array_Add` _wallneighbors_2 _output_2)
      (`KismetArrayLibrary.Array_Add` _wallneighbors_2 (`|GetArrayItem` (`self.SubWalls`) _returnvalue_2))
      (bind _returnvalue_3 (- _returnvalue_2 1))
      (`KismetArrayLibrary.Array_Add` _wallneighbors_2 (`|GetArrayItem` (`self.SubWalls`) (`KismetMathLibrary.SelectInt` _returnvalue_3 (+ _returnvalue (- (`self.Subdivision`) 1)) (`KismetArrayLibrary.Array_IsValidIndex` (`self.SubWalls`) _returnvalue_3))))
      (bind (_instanceindex _wallloc _pointa _pointb) (break `/Game/CircularLabyrinth/V1_BP/S_PROTO_Wall` _output))
      (`KismetArrayLibrary.Array_Add` _tempspoints _pointa)
      (`KismetArrayLibrary.Array_Add` _tempspoints _pointb)
      (bind (_instanceindex_2 _wallloc_2 _pointa_2 _pointb_2) (break `/Game/CircularLabyrinth/V1_BP/S_PROTO_Wall` _output_2))
      (`KismetArrayLibrary.Array_Add` _tempspoints _pointa_2)
      (`KismetArrayLibrary.Array_Add` _tempspoints _pointb_2)
      (`KismetArrayLibrary.Array_Add` (`self.Cells`) (make `/Game/CircularLabyrinth/V1_BP/S_PROTO_Cell` (+ (+ _index_2 _returnvalue) 1) (`KismetArrayLibrary.Array_Length` _wallneighbors) (/ (+ _wallloc _wallloc_2) 2.0) false false _wallneighbors (`self.TempsPoints`)))
      (`KismetArrayLibrary.Array_Clear` (`self.WallNeighbors`))
      (`KismetArrayLibrary.Array_Clear` (`self.TempsPoints`)))))

(fn `SetWallsPoints`
  (for _index (range (`self.CircleCount`))
    (for _index_2 (range (`self.Subdivision`))
      (bind _returnvalue (+ (* (`self.Subdivision`) _index) _index_2))
      (bind (_instanceindex _wallloc) (break `/Game/CircularLabyrinth/V1_BP/S_PROTO_Wall` (`|GetArrayItem` (`self.TempsWalls`) _returnvalue)))
      (`KismetArrayLibrary.Array_Add` (`self.CircleWalls`) (make `/Game/CircularLabyrinth/V1_BP/S_PROTO_Wall` _instanceindex _wallloc (`|GetArrayItem` (`self.GridPoints`) (`KismetMathLibrary.SelectInt` (- _returnvalue 1) (`KismetArrayLibrary.Array_LastIndex` (`self.GridPoints`)) (`KismetArrayLibrary.Array_IsValidIndex` (`self.GridPoints`) _returnvalue))) (`|GetArrayItem` (`self.GridPoints`) _returnvalue))))))

(fn `UserConstructionScript`
  (locals (`L Index` :type Integer))
  (`StaticMeshComponent.SetStaticMesh` (`self.HISM_Circle`) (`self.Static Mesh`))
  (`InstancedStaticMeshComponent.ClearInstances` (`self.HISM_Circle`))
  (`self.ClearVariables`)
  (`self.SetupCell_Index0`)
  (`self.DrawCircles&Points`)
  (`self.SetWallsPoints`)
  (`self.CreateWallsBetweenCircle&WallLoc`)
  (`self.SetWalls&PointsToCells`)
  (`self.DEBUG_CellTextIndex`)
  (`self.SetIndexCellsNeighbors`)
  (`self.FinalCellsSetup`))